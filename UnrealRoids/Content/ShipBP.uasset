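; ShipBP is a player-controlled ship that can thrust, turn and shoot.
; MoveForward input applies physics force to ShipCollider along its forward vector, while Turn input rotates the actor's forward vector around the Z axis by a fixed step per input event, without delta-time scaling.
; Shoot spawns a Bullet just ahead of the ship, facing the same direction.
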(event EventBeginPlay)

(event Collision|EventActorBeginOverlap
  (params (OtherActor :type Actor%20Object%20Reference)))

(event EventTick
  (params (DeltaSeconds :type Float%20%28single-precision%29)))

(event Input|ActionEvents|InputActionShoot
  (params (Key :type Key%20Structure :default "None"))
  (bind _returnvalue (Transformation|GetActorRotation))
  (:Pressed
    (Game|SpawnActorfromClass "/Game/Bullet.Bullet_C" (Math|Transform|MakeTransform (+ (Transformation|GetActorLocation) (* (Math|Vector|Normalize (Math|Vector|GetForwardVector _returnvalue)) 3e+01)) _returnvalue) "Undefined" 0 0)))

(event Input|AxisEvents|InputAxisMoveForward
  (params (AxisValue :type Float%20%28single-precision%29))
  (Physics|AddForce (Variables|Default|GetShipCollider) (* (Math|Vector|GetForwardVector (Variables|Default|GetShipCollider)) (* AxisValue 6e+02)) "None" false))

(event Input|AxisEvents|InputAxisTurn
  (params (AxisValue :type Float%20%28single-precision%29))
  (Transformation|SetActorRotation (Math|Rotator|MakeRotfromX (Math|Vector|RotateVectorAroundAxis (Math|Rotator|GetRotationXVector (Transformation|GetActorRotation)) (* AxisValue 4.0) "0, 0,1.000000"))))

(fn ConstructionScript)